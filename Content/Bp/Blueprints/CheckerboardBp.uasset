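; Board actor for a SameGame-style puzzle that fills a grid with randomly colored balls and frames it with an orthographic camera.
; SelectBalls uses a filtered breadth-first search to remove and score same-colored groups.
; A Tick-driven Status state machine then slides balls into gaps, closes emptied lines with lerped moves, and checks for remaining turns.
; An empty board wins and saves any new best score; no matches left loses.
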(event `self.ReceiveBeginPlay`
  (bind _size (`self.Size`))
  (bind _returnvalue (+ (`KismetMathLibrary.Conv_IntToDouble` (`self.Size`)) -0.5))
  (set `/Game/Bp/Blueprints/Global.Score` 0 (cast `/Game/Bp/Blueprints/Global` (`GameplayStatics.GetGameInstance`) :!pure true))
  (set `self.Status` "NewEnumerator0")
  (`KismetArrayLibrary.Array_Clear` (`self.Grid`))
  (`MeshComponent.SetScalarParameterValueOnMaterials` (`self.Plane`) "Size" (`KismetMathLibrary.Conv_IntToDouble` (`self.Size`)))
  (for _index (range (* _size _size 4))
    (bind (_x _y) (`self.Index to` _index))
    (bind _globalcoords (`self.To Position` (`KismetMathLibrary.Conv_IntToDouble` _x) (`KismetMathLibrary.Conv_IntToDouble` _y)))
    (bind _returnvalue_2 (`|SpawnActorFromClass` "/Game/Bp/Blueprints/ColorBall.ColorBall_C" (`KismetMathLibrary.MakeTransform` _globalcoords (struct) (/ (/ (`SceneComponent.K2_GetComponentScale` (`self.ChildActor`)) (`KismetMathLibrary.Conv_IntToDouble` (`self.Size`))) 2.2)) "AlwaysSpawn" "OverrideRootScale" self null))
    (`KismetArrayLibrary.Array_Insert` (`self.Grid`) _returnvalue_2 _index)
    (`/Game/Bp/Blueprints/ColorBall.SetColor` _returnvalue_2 (`|GetArrayItem` (`self.ColorsBalls`) (`KismetMathLibrary.RandomIntegerInRange` 0 (+ (`/Game/Bp/Blueprints/Global.Intricacy` (cast `/Game/Bp/Blueprints/Global` (`GameplayStatics.GetGameInstance`) :!pure true)) 2))))
    (`self.K2_AttachToActor` _returnvalue_2 self "None" "KeepWorld" "KeepWorld" "KeepWorld" true)
    (set `/Game/Bp/Blueprints/ColorBall.CheckerboardOwner` self _returnvalue_2)
    (set `self.Status` "NewEnumerator1"))
  (bind _globalcoords_2 (`self.To Position` _returnvalue _returnvalue -0.5))
  (`SceneComponent.K2_SetWorldLocation` (`self.Plane`) _globalcoords_2 false false)
  (`self.SetupCamera`))

(event `self.ReceiveTick`
  (params (DeltaSeconds :type "Float (single-precision)"))
  (switch `/Game/Bp/Blueprints/SatusGame` (`self.Status`)
    (:`NewEnumerator3`
      (bind _moves (`self.Сolumn`))
      (set `self.AnimationBalls` (make `/Game/Bp/Blueprints/MovementAnimation` _moves -1.0 -1.0)))
    (:`NewEnumerator4`
      (bind _moves_2 (`self.Row`))
      (set `self.AnimationBalls` (make `/Game/Bp/Blueprints/MovementAnimation` _moves_2 -1.0 -1.0)))
    (:`NewEnumerator2`
      (`self.ShiftBalls` :!label _label))
    (:`NewEnumerator5`
      (goto _label))
    (:`NewEnumerator8`
      (`self.CheckTurns`))))

(fn `CheckTurns`
  (locals (IsTurnExist :type Boolean) (IsNotEmpty :type Boolean))
  (bind _asglobal (cast `/Game/Bp/Blueprints/Global` (`GameplayStatics.GetGameInstance`) :!pure true))
  (bind _score (`/Game/Bp/Blueprints/Global.Score` _asglobal))
  (for _array_element (`self.Grid`)
    (`/Engine/EditorBlueprintResources/StandardMacros.IsValid` _array_element
      (:`Is Valid`
        (set `local.IsNotEmpty` true)
        (bind _returnvalue (`|GenericCreateObject` "/Game/Bp/Blueprints/ColorFilter.ColorFilter_C" "/Game/Bp/Blueprints/ColorFilter.ColorFilter"))
        (set `/Game/Bp/Blueprints/ColorFilter.Color` (`/Game/Bp/Blueprints/ColorBall.Color` _array_element) _returnvalue)
        (bind _neighbors (`self.Neighbors` _array_element -1 (`|MakeArray` _returnvalue :!type "/Game/Bp/Blueprints/IFilter Interface") (`self.Dir`)))
        (if (> (`KismetArrayLibrary.Array_Length` _neighbors) 1)
          (set `local.IsTurnExist` true)
          (break)))))
  (if (`local.IsNotEmpty`)
    (if (`local.IsTurnExist`)
      (set `self.Status` "NewEnumerator1")
      (else
        (set `self.Status` "NewEnumerator7")
        (bind _returnvalue_2 (`|CreateWidget` "/Game/Bp/Blueprints/UI/EndGame.EndGame_C"))
        (set `/Game/Bp/Blueprints/UI/EndGame.GameEnd` "NewEnumerator1" _returnvalue_2)
        (`UserWidget.AddToViewport` _returnvalue_2 0)))
    (else
      (set `self.Status` "NewEnumerator6")
      (bind _returnvalue_3 (`|CreateWidget` "/Game/Bp/Blueprints/UI/EndGame.EndGame_C"))
      (set `/Game/Bp/Blueprints/UI/EndGame.GameEnd` "NewEnumerator0" _returnvalue_3)
      (`UserWidget.AddToViewport` _returnvalue_3 0)
      (if (> _score (`/Game/Bp/Blueprints/Global.BestScore` _asglobal))
        (bind _output_get (set `/Game/Bp/Blueprints/Global.BestScore` _score _asglobal))
        (bind _assave_scores (cast `/Game/Bp/Blueprints/SaveScores` (`/Game/Bp/Blueprints/Global.SaveGame` _asglobal)))
        (`/Game/Bp/Blueprints/SaveScores.Save` _assave_scores _output_get)
        (`KismetSystemLibrary.PrintString` (`KismetStringLibrary.Conv_IntToString` _output_get) true true (struct :`R` 1.0 :`B` 0.078579 :`A` 1.0))))))

(fn `Factorial`
  (params (Int :type Integer))
  (returns (NewParam :type Integer))
  (locals (Fact :type Integer :default 1))
  (for _index (range 1 (+ Int 1))
    (set `local.Fact` (* (`local.Fact`) _index)))
  (return (`local.Fact`)))

(fn `Index to`
  (params (Index :type Integer))
  (returns (X :type Integer) (Y :type Integer))
  (bind _returnvalue (* (`self.Size`) 2))
  (return (mod Index _returnvalue) (/ Index _returnvalue)))

(fn `IsXYValid`
  (params (X :type Integer) (Y :type Integer))
  (returns (IsValid :type Boolean))
  (return (and (< X (* (`self.Size`) 2)) (< Y (* (`self.Size`) 2)) (>= X 0) (>= Y 0))))

(fn `Neighbors`
  (params (Ball :type "/Game/Bp/Blueprints/ColorBall Object Reference") (Range :type Integer :default -1) (Filters :type "Array of /Game/Bp/Blueprints/IFilter Interface") (MoveDirections :type "Array of IntVector Structure (by ref)"))
  (returns (Neighbors :type "Array of /Game/Bp/Blueprints/QueueBallElement Structure"))
  (locals (Queue :type "Array of /Game/Bp/Blueprints/QueueBallElement Structure") (Ans :type "Array of /Game/Bp/Blueprints/QueueBallElement Structure") (Visited :type "Array of Boolean") (FilterValue :type Boolean))
  (bind (_output_ball _output_length _output_x _output_y) (break `/Game/Bp/Blueprints/QueueBallElement` (`|GetArrayItem` (`local.Queue`))))
  (for _ (`self.Grid`)
    (`KismetArrayLibrary.Array_Add` (`local.Visited`)))
  (bind (_x _y) (`self.Position To` (`self.K2_GetActorLocation` Ball)))
  (bind _index (`self.To Index` _x _y))
  (`KismetArrayLibrary.Array_Set` (`local.Visited`) _index true)
  (`KismetArrayLibrary.Array_Add` (`local.Queue`) (make `/Game/Bp/Blueprints/QueueBallElement` Ball 0 _x _y))
  (while (> (`KismetArrayLibrary.Array_Length` (`local.Queue`)) 0)
    (if (or (> Range _output_length) (== Range -1))
      (for _array_element MoveDirections
        (bind _returnvalue (+ _output_x (break `IntVector` _array_element)))
        (bind _returnvalue_2 (+ _output_y (`.Y` (break `IntVector` _array_element))))
        (bind _index_2 (`self.To Index` _returnvalue _returnvalue_2))
        (bind _isvalid (`self.IsXYValid` _returnvalue _returnvalue_2))
        (if (and (not (`|GetArrayItem` (`local.Visited`) _index_2)) _isvalid)
          (`KismetArrayLibrary.Array_Set` (`local.Visited`) _index_2 true)
          (bind _output (`|GetArrayItem` (`self.Grid`) _index_2))
          (`/Engine/EditorBlueprintResources/StandardMacros.IsValid` _output
            (:`Is Valid`
              (set `local.FilterValue` true)
              (for _array_element_2 Filters
                (bind _isfit (`/Game/Bp/Blueprints/IFilter.Check` _array_element_2 _output))
                (bind _output_get (set `local.FilterValue` (and _isfit (`local.FilterValue`)))))
              (if _output_get
                (`KismetArrayLibrary.Array_Add` (`local.Queue`) (make `/Game/Bp/Blueprints/QueueBallElement` _output (+ _output_length 1) _returnvalue _returnvalue_2))))))))
    (`KismetArrayLibrary.Array_Add` (`local.Ans`) (`|GetArrayItem` (`local.Queue`)))
    (`KismetArrayLibrary.Array_Remove` (`local.Queue`)))
  (return (`local.Ans`)))

(fn `Position To`
  (params (GlobalCoords :type "Vector Structure"))
  (returns (X :type Integer) (Y :type Integer) (NewParam :type "Vector Structure"))
  (bind (_returnvalue_x _returnvalue_y) (`KismetMathLibrary.BreakVector` (/ (`KismetMathLibrary.InverseTransformLocation` (`self.GetTransform` self) GlobalCoords) (/ (`self.SizePanel`) (`KismetMathLibrary.Conv_IntToDouble` (* (`self.Size`) 2))))))
  (return (`KismetMathLibrary.Round` _returnvalue_x) (`KismetMathLibrary.Round` _returnvalue_y) (0.0 0.0 0.0)))

(fn `Row`
  (returns (Moves :type "Array of /Game/Bp/Blueprints/IntVectorPair Structure"))
  (locals (MovesList :type "Array of /Game/Bp/Blueprints/IntVectorPair Structure") (X :type Integer) (Y :type Integer))
  (bind _x (`local.X`))
  (bind _returnvalue (- (* (`self.Size`) 2) 1))
  (for _index (range 1 (+ _returnvalue 1))
    (bind _output_get (set `local.Y` _index))
    (bind _returnvalue_2 (- _output_get 1))
    (bind _isvalid (`self.IsXYValid` 0 _returnvalue_2))
    (if _isvalid
      (bind _index_2 (`self.To Index` 0 _returnvalue_2))
      (`/Engine/EditorBlueprintResources/StandardMacros.IsValid` (`|GetArrayItem` (`self.Grid`) _index_2)
        (:`Is Not Valid`
          (for _index_3 (range (+ _returnvalue 1))
            (bind _output_get_2 (set `local.X` _index_3))
            (bind _index_4 (`self.To Index` _output_get_2 (`local.Y`)))
            (`/Engine/EditorBlueprintResources/StandardMacros.IsValid` (`|GetArrayItem` (`self.Grid`) _index_4)
              (:`Is Valid`
                (`KismetArrayLibrary.Array_Add` (`local.MovesList`) (make `/Game/Bp/Blueprints/IntVectorPair` (make `IntVector` _x (`local.Y`)) (make `IntVector` _x _returnvalue_2))))
              (:`Is Not Valid`
                (break))))))))
  (if (> (`KismetArrayLibrary.Array_Length` (`local.MovesList`)) 0)
    (set `self.Status` "NewEnumerator5")
    (else
      (set `self.Status` "NewEnumerator8")))
  (return (`local.MovesList`)))

(fn `SelectBalls`
  (params (Ball :type "/Game/Bp/Blueprints/ColorBall Object Reference"))
  (locals (F :type "/Game/Bp/Blueprints/ColorFilter Object Reference"))
  (bind _asglobal (cast `/Game/Bp/Blueprints/Global` (`GameplayStatics.GetGameInstance`) :!pure true))
  (if (`|EnumEquality` (`self.Status`) "NewEnumerator1")
    (bind _returnvalue (`|GenericCreateObject` "/Game/Bp/Blueprints/ColorFilter.ColorFilter_C" "/Game/Bp/Blueprints/ColorFilter.ColorFilter"))
    (bind _color (`/Game/Bp/Blueprints/ColorBall.GetColor` Ball))
    (set `/Game/Bp/Blueprints/ColorFilter.Color` _color _returnvalue)
    (bind _neighbors (`self.Neighbors` Ball -1 (`|MakeArray` _returnvalue :!type "/Game/Bp/Blueprints/IFilter Interface") (`self.Dir`)))
    (bind _returnvalue_2 (`KismetArrayLibrary.Array_Length` _neighbors))
    (if (> _returnvalue_2 1)
      (bind _returnvalue_3 (+ (* _returnvalue_2 (+ (* (`/Game/Bp/Blueprints/Global.Intricacy` _asglobal) 5) 10)) (/ (`self.Factorial` _returnvalue_2) (`self.Factorial` (/ _returnvalue_2 2)))))
      (set `/Game/Bp/Blueprints/Global.Score` (+ _returnvalue_3 (`/Game/Bp/Blueprints/Global.Score` _asglobal)) _asglobal)
      (`KismetSystemLibrary.PrintString` (`KismetStringLibrary.Conv_IntToString` _returnvalue_3))
      (for _array_element _neighbors
        (`self.K2_DestroyActor` (break `/Game/Bp/Blueprints/QueueBallElement` _array_element))
        (bind _index (`self.To Index` (`.X_8_26A6745F42A7FC42BB20B7B0743F0D9A` (break `/Game/Bp/Blueprints/QueueBallElement` _array_element)) (`.Y_10_9B2AC7CE4DC30C867E177EA06602D192` (break `/Game/Bp/Blueprints/QueueBallElement` _array_element))))
        (`KismetArrayLibrary.Array_Set` (`self.Grid`) _index)
        (set `self.Status` "NewEnumerator3")))))

(fn `SetupCamera`
  (bind _camera (`self.Camera`))
  (bind _cameracomponent (`CameraActor.CameraComponent` (`self.Camera`)))
  (bind _returnvalue (+ (`KismetMathLibrary.Conv_IntToDouble` (`self.Size`)) -0.5))
  (bind (_returnvalue_x _returnvalue_y) (`KismetMathLibrary.BreakVector` (* (`self.SizePanel`) (`self.GetActorScale3D` self))))
  (bind _globalcoords (`self.To Position` _returnvalue _returnvalue -0.5))
  (`/Engine/EditorBlueprintResources/StandardMacros.IsValid` _camera
    (:`Is Valid`
      (`SceneComponent.K2_SetWorldLocation` (`Actor.RootComponent` _camera) (+ _globalcoords (0.0 0.0 100.0)) false false)
      (`CameraComponent.SetProjectionMode` _cameracomponent "Orthographic")
      (`CameraComponent.SetAspectRatio` _cameracomponent 1.0)
      (`CameraComponent.SetOrthoWidth` _cameracomponent (`KismetMathLibrary.FMax` _returnvalue_x _returnvalue_y)))))

(fn `ShiftBalls`
  (bind _returnvalue (`self.GetGameTimeSinceCreation`))
  (bind _returnvalue_2 (`self.GetGameTimeSinceCreation`))
  (bind _animationballs_moves (break `/Game/Bp/Blueprints/MovementAnimation` (`self.AnimationBalls`)))
  (bind _grid (`self.Grid`))
  (bind (_animationballs_moves_2 _animationballs_starttime _animationballs_endtime) (break `/Game/Bp/Blueprints/MovementAnimation` (`self.AnimationBalls`)))
  (bind (_moves _starttime) (break `/Game/Bp/Blueprints/MovementAnimation` (`self.AnimationBalls`)))
  (if (`KismetMathLibrary.NearlyEqual_FloatFloat` _starttime -1.0)
    (bind _output_get (set `self.AnimationBalls` (make `/Game/Bp/Blueprints/MovementAnimation` _moves _returnvalue_2 (+ _returnvalue_2 (`self.SpeedAnim`))))))
  (for _array_element (break `/Game/Bp/Blueprints/MovementAnimation` _output_get)
    (bind _index (`self.To Index` (break `IntVector` (break `/Game/Bp/Blueprints/IntVectorPair` _array_element)) (`.Y` (break `IntVector` (break `/Game/Bp/Blueprints/IntVectorPair` _array_element)))))
    (bind (_returnvalue_x _returnvalue_y) (`KismetMathLibrary.BreakVector` (`KismetMathLibrary.VLerp` (`KismetMathLibrary.MakeVector` (`KismetMathLibrary.Conv_IntToDouble` (break `IntVector` (break `/Game/Bp/Blueprints/IntVectorPair` _array_element))) (`KismetMathLibrary.Conv_IntToDouble` (`.Y` (break `IntVector` (break `/Game/Bp/Blueprints/IntVectorPair` _array_element))))) (`KismetMathLibrary.MakeVector` (`KismetMathLibrary.Conv_IntToDouble` (break `IntVector` (`.Second_5_2C9841004C2727A4ECBDDCAFA1A30996` (break `/Game/Bp/Blueprints/IntVectorPair` _array_element)))) (`KismetMathLibrary.Conv_IntToDouble` (`.Y` (break `IntVector` (`.Second_5_2C9841004C2727A4ECBDDCAFA1A30996` (break `/Game/Bp/Blueprints/IntVectorPair` _array_element)))))) (`KismetMathLibrary.FMin` (/ (- _returnvalue _animationballs_starttime) (- _animationballs_endtime _animationballs_starttime)) 1.0))))
    (bind _globalcoords (`self.To Position` _returnvalue_x _returnvalue_y))
    (`self.K2_SetActorLocation` (`|GetArrayItem` (`self.Grid`) _index) _globalcoords false false))
  (if (>= _returnvalue _animationballs_endtime)
    (switch `/Game/Bp/Blueprints/SatusGame` (`self.Status`)
      (:`NewEnumerator2`
        (set `self.Status` "NewEnumerator3"))
      (:`NewEnumerator5`
        (set `self.Status` "NewEnumerator4")))
    (for _array_element_2 _animationballs_moves
      (bind _index_2 (`self.To Index` (break `IntVector` (break `/Game/Bp/Blueprints/IntVectorPair` _array_element_2)) (`.Y` (break `IntVector` (break `/Game/Bp/Blueprints/IntVectorPair` _array_element_2)))))
      (bind _index_3 (`self.To Index` (break `IntVector` (`.Second_5_2C9841004C2727A4ECBDDCAFA1A30996` (break `/Game/Bp/Blueprints/IntVectorPair` _array_element_2))) (`.Y` (break `IntVector` (`.Second_5_2C9841004C2727A4ECBDDCAFA1A30996` (break `/Game/Bp/Blueprints/IntVectorPair` _array_element_2))))))
      (`KismetArrayLibrary.Array_Set` _grid _index_3 (`|GetArrayItem` _grid _index_2))
      (`KismetArrayLibrary.Array_Set` _grid _index_2))))

(fn `To Index`
  (params (X :type Integer) (Y :type Integer))
  (returns (Index :type Integer))
  (return (+ X (* Y (* (`self.Size`) 2)))))

(fn `To Position`
  (params (X :type "Float (double-precision)") (Y :type "Float (double-precision)") (Z :type "Float (double-precision)"))
  (returns (GlobalCoords :type "Vector Structure"))
  (return (`KismetMathLibrary.TransformLocation` (`self.GetTransform` self) (* (`KismetMathLibrary.MakeVector` X Y Z) (/ (`self.SizePanel`) (`KismetMathLibrary.Conv_IntToDouble` (* (`self.Size`) 2)))))))

(fn `UserConstructionScript`)

(fn `Сolumn`
  (returns (Moves :type "Array of /Game/Bp/Blueprints/IntVectorPair Structure"))
  (locals (MovesList :type "Array of /Game/Bp/Blueprints/IntVectorPair Structure") (Y :type Integer) (X :type Integer))
  (bind _y (`local.Y`))
  (bind _returnvalue (- (* (`self.Size`) 2) 1))
  (for _index (range (+ _returnvalue 1))
    (set `local.Y` _index)
    (for _index_2 (range 1 (+ _returnvalue 1))
      (bind _output_get (set `local.X` _index_2))
      (bind _index_3 (`self.To Index` (`local.X`) (`local.Y`)))
      (`/Engine/EditorBlueprintResources/StandardMacros.IsValid` (`|GetArrayItem` (`self.Grid`) _index_3)
        (:`Is Valid`
          (bind _returnvalue_2 (+ _output_get -1))
          (bind _isvalid (`self.IsXYValid` _returnvalue_2 (`local.Y`)))
          (if _isvalid
            (bind _index_4 (`self.To Index` _returnvalue_2 (`local.Y`)))
            (`/Engine/EditorBlueprintResources/StandardMacros.IsValid` (`|GetArrayItem` (`self.Grid`) _index_4)
              (:`Is Not Valid`
                (`KismetArrayLibrary.Array_Add` (`local.MovesList`) (make `/Game/Bp/Blueprints/IntVectorPair` (make `IntVector` (`local.X`) _y) (make `IntVector` _returnvalue_2 _y))))))))))
  (if (> (`KismetArrayLibrary.Array_Length` (`local.MovesList`)) 0)
    (set `self.Status` "NewEnumerator2")
    (else
      (set `self.Status` "NewEnumerator4")))
  (return (`local.MovesList`)))