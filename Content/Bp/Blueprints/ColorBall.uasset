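; ColorBall is a colored sphere piece that belongs to a checkerboard and can be picked by click or touch.
; It starts white, and SetColor stores the color and writes it to the Sphere's "Color" material parameter, with GetColor returning the stored value.
; Releasing a click or ending a touch on the Sphere passes the ball to its CheckerboardOwner through SelectBalls.
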(event `self.ReceiveBeginPlay`
  (`self.SetColor` (1.0 1.0 1.0)))

(event `self.Sphere.OnReleased`
  (params (TouchedComponent :type "PrimitiveComponent Object Reference") (ButtonReleased :type "Key Structure"))
  (`/Game/Bp/Blueprints/CheckerboardBp.SelectBalls` (`self.CheckerboardOwner`) self :!label _label))

(event `self.Sphere.OnInputTouchEnd`
  (params (FingerIndex :type "ETouchIndex Enum" :default "Touch1") (TouchedComponent :type "PrimitiveComponent Object Reference"))
  (goto _label))

(fn `GetColor`
  (returns (Color :type "Vector Structure"))
  (return (`self.Color`)))

(fn `SetColor`
  (params (Color :type "Vector Structure"))
  (bind _output_get (set `self.Color` Color))
  (`MeshComponent.SetVectorParameterValueOnMaterials` (`self.Sphere`) "Color" _output_get))

(fn `UserConstructionScript`)